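; Gameplay ability that dashes the Sage player along last movement input, or facing direction when idle, while playing a montage.
; FindFarthestLocation steps back from maximum range in capsule-diameter increments until a spot has ground below and no Pawn-blocking overlap.
; A timeline lerps the avatar there without sweeping, so it can pass through obstacles.
; The ability ends on montage completion and calls CommitAbility only in OnEndAbility.
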(event Custom|MoveOverTime
  (params (TargetLocation :type Vector))
  (bind _returnvalue (Ability|GetAvatarActorfromActorInfo))
  (bind _output_get (Variables|Default|SetStartLocation (Transformation|GetActorLocation _returnvalue)))
  (Transformation|SetActorRotation _returnvalue (Math|Rotator|FindLookatRotation _output_get TargetLocation))
  (bind _value (|FloatTimeline)
    (:OnUpdate
      (Transformation|SetActorLocation _returnvalue (Math|Vector|Lerp(Vector) (Variables|Default|GetStartLocation) TargetLocation _value) false false))))

(event Ability|EventActivateAbility
  (bind _returnvalue (Ability|GetAvatarActorfromActorInfo))
  (bind _finallocation (CallFunction|CalCulateFinalLocation))
  (bind _returnvalue_2 (Transformation|GetActorLocation _returnvalue))
  (bind _farthest_location (CallFunction|FindFarthestLocation _returnvalue_2 _finallocation))
  (|PlayMontageandWaitProxy "None" "/Game/Bluprints/Animation/CustomAnim/AM_Dash.AM_Dash" 1.0 "None" true 1.0 0.0 false
    (:then
      (if (not (Utilities|Operators|EqualEqual _farthest_location _returnvalue_2 1.0))
        (CallFunction|MoveOverTime _farthest_location)))
    (:OnCompleted
      (Ability|EndAbility))))

(event Ability|EventOnEndAbility
  (params (bWasCancelled :type Boolean))
  (Ability|CommitAbility))

(fn FindFarthestLocation
  (params (StartLocation :type Vector) (EndLocation :type Vector))
  (LocalVariables|SetDirection (Math|Vector|GetUnitDirection(Vector) StartLocation EndLocation))
  (bind _asbp_sage_player (Utilities|Casting|CastToBP_SagePlayer (Game|GetPlayerCharacter 0)))
  (bind _output_get (LocalVariables|SetCapsuleDiameter (* (Components|Capsule|GetScaledCapsuleRadius (Variables|/Script/Engine.Character|GetCapsuleComponent _asbp_sage_player)) 2.0)))
  (bind _output_get_2 (LocalVariables|SetCapsuleAmount (/ (Math|Vector|Distance(Vector) StartLocation EndLocation) _output_get)))
  (for _index (range 0 _output_get_2)
    (LocalVariables|SetLastLoopLocation (+ (* (- (LocalVariables|GetCapsuleAmount) _index) (LocalVariables|GetDirection) (LocalVariables|GetCapsuleDiameter)) StartLocation))
    (bind _outhits (Class|KismetSystemLibrary|CapsuleTraceMultiforObjects (+ (* (- (LocalVariables|GetCapsuleAmount) _index) (LocalVariables|GetDirection) (LocalVariables|GetCapsuleDiameter)) StartLocation) (+ (* (- (LocalVariables|GetCapsuleAmount) _index) (LocalVariables|GetDirection) (LocalVariables|GetCapsuleDiameter)) StartLocation) (.OutRadius (Class|CapsuleComponent|GetUnscaledCapsuleSize (Variables|/Script/Engine.Character|GetCapsuleComponent _asbp_sage_player))) (.OutHalfHeight (Class|CapsuleComponent|GetUnscaledCapsuleSize (Variables|/Script/Engine.Character|GetCapsuleComponent _asbp_sage_player))) (Utilities|Array|MakeArray "ObjectTypeQuery1" "ObjectTypeQuery2" "ObjectTypeQuery3" "ObjectTypeQuery6" "ObjectTypeQuery5") false 0 "None" true))
    (bind _is_valid (CallFunction|IsThisLocationValid (LocalVariables|GetLastLoopLocation) _outhits))
    (if _is_valid
      (return (LocalVariables|GetLastLoopLocation))))
  (return StartLocation))

(fn IsThisLocationValid
  (params (Location :type Vector) (NewParam :type Array%20of%20Hit%20Result%20Structures))
  (bind _returnvalue (Collision|LineTraceByChannel Location (+ Location "0.000000,0.000000,-500.000000") "TraceTypeQuery1" false 0 "None"))
  (if _returnvalue
    (if (Utilities|Array|IsEmpty NewParam)
      (return true)
      (else
        (for _array_element NewParam
          (if (Utilities|Enum|Equal(Enum) (Collision|GetCollisionResponsetoChannel (.HitComponent (Collision|BreakHitResult _array_element)) "ECC_Pawn") "ECR_Block")
            (return false)))
        (return true)))
    (else
      (return false))))

(fn CalCulateFinalLocation
  (bind _asbp_sage_player (Utilities|Casting|CastToBP_SagePlayer (Game|GetPlayerCharacter 0)))
  (return (+ (Transformation|GetActorLocation _asbp_sage_player) (* (Math|Vector|SelectVector (Transformation|GetActorForwardVector _asbp_sage_player) (Pawn|Components|PawnMovement|GetLastInputVector (Variables|/Script/Engine.Character|GetCharacterMovement _asbp_sage_player)) (Utilities|Operators|EqualEqual :A (Pawn|Components|PawnMovement|GetLastInputVector (Variables|/Script/Engine.Character|GetCharacterMovement _asbp_sage_player)))) (Variables|Default|GetMaxDashTarget)))))